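; Top-down camera controller that pans and zooms a camera pawn and directs the Builder character by mouse.
; Axis input and a screen-edge scroller macro move the pawn, the mouse wheel adjusts clamped spring-arm length, and SpaceBar recenters on the Builder.
; While click is held, a gated Tick sends cursor hits to AI navigation if distant enough, within map bounds and the Builder isn't mining or chopping.
; BeginPlay caches references, shows the cursor and creates the UI.
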(event EventBeginPlay
  ;[1 1 1] Referencing
  (Utilities|FlowControl|Sequence
    (:then_0
      (Utilities|HandleReferences))
    (:then_1
      (Variables|/Script/Engine.PlayerController|SetbShowMouseCursor (Game|GetPlayerController 0) true))
    (:then_2
      (bind _outactors (Actor|GetAllActorsOfClass "/Script/Engine.Character"))
      (Variables|References|SetBuilderRef (Utilities|Array|Get(acopy) _outactors)))
    (:then_3
      (Utilities|SetupUI))
    (:then_4
      (CallFunction|FocusPlayer))))

(event EventTick
  (params (DeltaSeconds :type Float%20%28single-precision%29))
  (bind _hitresult (Game|Player|GetHitResultUnderCursorbyChannel "TraceTypeQuery1" true))
  (bind _location (Collision|BreakHitResult _hitresult))
  (bind (_x _y _z) (Math|Vector|BreakVector _location))
  ;[1 1 1] Builder Character Movement
  (Utilities|FlowControl|Gate true
    (:Exit
      (bind _asbuilder (Utilities|Casting|CastToBuilder (Variables|References|GetBuilderRef)))
      (if (Math|Boolean|ANDBoolean (>= (Math|Vector|VectorLength (- (Transformation|GetActorLocation (Variables|References|GetBuilderRef)) _location)) (Variables|Default|GetMinClickDistance)) (Math|Boolean|ANDBoolean (<= _x 4e+03) (>= _x -4e+03) (<= _y 4e+03) (>= _y -4e+03) (<= _z 7e+02)) (and (not (Variables|/Game/Blueprints/Builder.Builder_C|GetisMining _asbuilder)) (not (Variables|/Game/Blueprints/Builder.Builder_C|GetisChoppingTree _asbuilder))))
        (CallFunction|MoveBuilder _hitresult)
        (else
          (Development|PrintString "Location is out of reach!" true true "(R=1.000000,G=0.000000,B=0.000000,A=1.000000)"))))))

(event Input|ActionEvents|InputActionMouseClick
  (params (Key :type Key%20Structure))
  (bind _hitresult (Game|Player|GetHitResultUnderCursorbyChannel "TraceTypeQuery1" true))
  (bind _location (Collision|BreakHitResult _hitresult))
  (bind (_x _y _z) (Math|Vector|BreakVector _location))
  ;[1 1 1] Builder Character Movement
  (:Pressed
    (Utilities|FlowControl|Gate true) ; enters at Open
  )
  (:Released
    (Utilities|FlowControl|Gate true) ; enters at Close
  ))

(event Input|AxisEvents|InputAxisForward/Backward
  (params (AxisValue :type Float%20%28single-precision%29))
  ;[1 1 1] Control the Camera with keyboard
  (CallFunction|Movement 0.0 AxisValue))

(event Input|AxisEvents|InputAxisRight/Left
  (params (AxisValue :type Float%20%28single-precision%29))
  ;[1 1 1] Control the Camera with keyboard
  (CallFunction|Movement AxisValue 0.0))

(event Input|MouseEvents|MouseX
  (params (AxisValue :type Float%20%28single-precision%29))
  ;[1 1 1] Screen Edge Scrolling
  (bind (_speedx _speedy) (Utilities|ScreenEdgeScroller))
  (Transformation|AddActorLocalOffset (Variables|References|GetCameraPawnRef) (Math|Vector|MakeVector _speedx _speedy 0.0) false false))

(event Input|MouseEvents|MouseY
  (params (AxisValue :type Float%20%28single-precision%29))
  ;[1 1 1] Screen Edge Scrolling
  (Utilities|ScreenEdgeScroller) ; enters at MouseY
)

(event Input|MouseEvents|MouseWheelAxis
  (params (AxisValue :type Float%20%28single-precision%29))
  (bind _camerapawnref (Variables|References|GetCameraPawnRef))
  (bind _springarm (Variables|/Game/Blueprints/CameraPawn.CameraPawn_C|GetSpringArm _camerapawnref))
  ;[1 1 1] Zoom In / Out
  (Variables|/Script/Engine.SpringArmComponent|SetTargetArmLength _springarm (Math|Float|Clamp(Float) (+ (Variables|/Script/Engine.SpringArmComponent|GetTargetArmLength _springarm) (* AxisValue (Variables|Default|GetScrollSpeed))) 5e+02 2e+03)))

(event Input|KeyboardEvents|SpaceBar
  (params (Key :type Key%20Structure))
  ;[1 1 1] Character Focus
  (:Pressed
    (CallFunction|FocusPlayer)))

(fn ConstructionScript)

(fn Movement
  (params (Horizontal :type Float%20%28single-precision%29) (Vertical :type Float%20%28single-precision%29))
  (bind _camerapawnref (Variables|References|GetCameraPawnRef))
  (bind _camspeed (Variables|Default|GetCamSpeed))
  (bind _returnvalue (Transformation|GetActorLocation _camerapawnref))
  (Transformation|SetActorLocation _camerapawnref (Math|Vector|MakeVector (Math|Float|Clamp(Float) (+ (.x _returnvalue) (* Vertical _camspeed)) -3e+03 3e+03) (Math|Float|Clamp(Float) (+ (.y _returnvalue) (* Horizontal _camspeed)) -4e+03 4e+03) (.z _returnvalue)) false false))

(fn MoveBuilder
  (params (Hit :type Hit%20Result%20Structure))
  (bind _location (Collision|BreakHitResult Hit))
  (if (>= (Math|Vector|VectorLength (- (Transformation|GetActorLocation (Variables|References|GetBuilderRef)) _location)) 2e+02) ; Don't move if player clicks too close to pawn
    (bind _asbuilder (Utilities|Casting|CastToBuilder (Variables|References|GetBuilderRef)))
    (Variables|/Game/Blueprints/Builder.Builder_C|SetGoalLocation _asbuilder _location)
    (AI|Navigation|SimpleMovetoLocation (AI|GetAIController (Variables|References|GetBuilderRef)) _location)))

(fn FocusPlayer
  (bind _camerapawnref (Variables|References|GetCameraPawnRef))
  (bind _builderref (Variables|References|GetBuilderRef))
  (bind _returnvalue (Transformation|GetActorLocation _builderref))
  (Transformation|SetActorLocation _camerapawnref (Math|Vector|MakeVector (.x _returnvalue) (.y _returnvalue) (.z (Transformation|GetActorLocation _camerapawnref))) false false)
  (return))