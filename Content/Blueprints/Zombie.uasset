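; Enemy zombie character that runs to the Tree of Life and attacks it until killed by bullets.
; Tick steers it via AI move-to until within attack range, then stops it and damages the tree on a delay set by attack speed.
; Bullet overlaps reduce hit points and refresh a health bar widget that turns toward the camera pawn each frame.
; State changes set ZombieAnimBP flags, and death plays out briefly before the actor is destroyed.
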(event OnComponentBeginOverlap(CapsuleComponent)
  (params (OverlappedComponent :type Primitive%20Component%20Object%20Reference) (OtherActor :type Actor%20Object%20Reference) (OtherComp :type Primitive%20Component%20Object%20Reference) (OtherBodyIndex :type Integer) (bFromSweep :type Boolean) (SweepResult :type Hit%20Result%20Structure%20%28by%20ref%29))
  ;[1 1 1] Getting hit
  (bind _asbullet (Utilities|Casting|CastToBullet OtherActor))
  (CallFunction|GetHit (Variables|/Game/Blueprints/Buildings/Defense/Bullet.Bullet_C|GetBulletDamage _asbullet))
  (if (<= (Variables|Default|GetHitPoints) 0.0)
    (CallFunction|OnDeath)
    (Utilities|FlowControl|Delay 2.5)
    (Actor|DestroyActor)))

(event OnComponentEndOverlap(CapsuleComponent)
  (params (OverlappedComponent :type Primitive%20Component%20Object%20Reference) (OtherActor :type Actor%20Object%20Reference) (OtherComp :type Primitive%20Component%20Object%20Reference) (OtherBodyIndex :type Integer))
  ;[1 1 1] Getting hit
  (bind _asbullet (Utilities|Casting|CastToBullet OtherActor))
  (Actor|DestroyActor _asbullet))

(event EventBeginPlay
  ;[1 1 1] References & Updating the UI
  (bind _outactors (Actor|GetAllActorsOfClass "/Game/Blueprints/TreeOfLife.TreeOfLife_C"))
  (bind _output_get (Variables|Default|SetTarget (Utilities|Array|Get(acopy) _outactors)))
  (Variables|Default|SetGoalLocation (Transformation|GetActorLocation _output_get))
  (bind _outactors_2 (Actor|GetAllActorsOfClass "/Game/Blueprints/CameraPawn.CameraPawn_C"))
  (Variables|Default|SetCameraPawn (Utilities|Array|Get(acopy) _outactors_2))
  (CallFunction|UpdateHpBarUI))

(event EventTick
  (params (DeltaSeconds :type Float%20%28single-precision%29))
  ;[1 1 1] Move to target & Attack
  (CallFunction|MoveHPBar)
  (if (> (Math|Vector|VectorLength (- (Transformation|GetActorLocation (Variables|Default|GetTarget)) (Transformation|GetActorLocation self))) (Variables|Default|GetAttackDistance))
    (CallFunction|MoveZombie)
    (else
      (CallFunction|StopZombie)
      (if (> (Variables|Default|GetHitPoints) 0.0)
        (Utilities|FlowControl|Delay (/ 1.0 (Variables|Default|GetAttackSpeed)))
        (CallFunction|Attack)))))

(fn ConstructionScript)

(fn MoveZombie
  (bind _aszombie_anim_bp (Utilities|Casting|CastToZombieAnimBP (Components|SkeletalMesh|GetAnimInstance (Variables|Character|GetMesh))))
  (Variables|/Game/Zombie/ZombieAnimBP.ZombieAnimBP_C|SetisIdle _aszombie_anim_bp false)
  (Variables|/Game/Zombie/ZombieAnimBP.ZombieAnimBP_C|SetisRunning _aszombie_anim_bp true)
  (Variables|/Game/Zombie/ZombieAnimBP.ZombieAnimBP_C|SetisAttacking _aszombie_anim_bp false)
  (AI|Navigation|SimpleMovetoLocation (AI|GetAIController self) (Variables|Default|GetGoalLocation))
  (return))

(fn StopZombie
  (Components|Movement|StopMovementImmediately (Variables|Character|GetCharacterMovement))
  (bind _aszombie_anim_bp (Utilities|Casting|CastToZombieAnimBP (Components|SkeletalMesh|GetAnimInstance (Variables|Character|GetMesh))))
  (Variables|/Game/Zombie/ZombieAnimBP.ZombieAnimBP_C|SetisIdle _aszombie_anim_bp true)
  (Variables|/Game/Zombie/ZombieAnimBP.ZombieAnimBP_C|SetisRunning _aszombie_anim_bp false)
  (return))

(fn Attack
  (bind _astree_of_life (Utilities|Casting|CastToTreeOfLife (Variables|Default|GetTarget)))
  (Default|GetDamaged _astree_of_life (Variables|Default|GetDamage))
  (bind _aszombie_anim_bp (Utilities|Casting|CastToZombieAnimBP (Components|SkeletalMesh|GetAnimInstance (Variables|Character|GetMesh))))
  (Variables|/Game/Zombie/ZombieAnimBP.ZombieAnimBP_C|SetisIdle _aszombie_anim_bp false)
  (Variables|/Game/Zombie/ZombieAnimBP.ZombieAnimBP_C|SetisRunning _aszombie_anim_bp false)
  (Variables|/Game/Zombie/ZombieAnimBP.ZombieAnimBP_C|SetisAttacking _aszombie_anim_bp true)
  (return))

(fn GetHit
  (params (Damage :type Float%20%28single-precision%29))
  (Variables|Default|SetHitPoints (- (Variables|Default|GetHitPoints) Damage))
  (CallFunction|UpdateHpBarUI)
  (return))

(fn OnDeath
  (bind _aszombie_anim_bp (Utilities|Casting|CastToZombieAnimBP (Components|SkeletalMesh|GetAnimInstance (Variables|Character|GetMesh))))
  (CallFunction|StopZombie)
  (Variables|/Game/Zombie/ZombieAnimBP.ZombieAnimBP_C|SetisAttacking _aszombie_anim_bp false)
  (Variables|/Game/Zombie/ZombieAnimBP.ZombieAnimBP_C|SetisIdle _aszombie_anim_bp false)
  (Variables|/Game/Zombie/ZombieAnimBP.ZombieAnimBP_C|SetisDead _aszombie_anim_bp true)
  (return))

(fn MoveHPBar
  (bind _hpbar (Variables|Default|GetHPBar))
  (bind _ascamera_pawn (Utilities|Casting|CastToCameraPawn (Variables|Default|GetCameraPawn)))
  (Transformation|SetWorldRotation _hpbar (Math|Rotator|FindLookatRotation (Transformation|GetWorldLocation _hpbar) (Transformation|GetWorldLocation (Components|GetChildComponent (Variables|/Game/Blueprints/CameraPawn.CameraPawn_C|GetCamera _ascamera_pawn) 0))) false false))

(fn UpdateHpBarUI
  (bind _aszombie_hpbar (Utilities|Casting|CastToZombieHPBar (UserInterface|GetUserWidgetObject (Variables|Default|GetHPBar))))
  (Default|GetHealthPercentage _aszombie_hpbar (Math|Float|NormalizetoRange (/ (Variables|Default|GetHitPoints) (Variables|Default|GetMaxHP)) 0.0 1.0))
  (return))