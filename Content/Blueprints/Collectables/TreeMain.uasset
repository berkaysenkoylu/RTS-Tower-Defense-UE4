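; Collectable tree actor that lets the Builder character chop it, with debug prints for the facing check.
; Collider overlap enables input and compares the actor's forward vector to the tree's direction by dot product against an offset, once on entry.
; Right mouse sets the Builder's chopping state when in reach and facing; leaving clears it.
; Clicking ClickSurface calls TreeChoppingAction on the first Character found at BeginPlay, without those checks.
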(event OnComponentBeginOverlap(TreeMainCollider)
  (params (OverlappedComponent :type Primitive%20Component%20Object%20Reference) (OtherActor :type Actor%20Object%20Reference) (OtherComp :type Primitive%20Component%20Object%20Reference) (OtherBodyIndex :type Integer) (bFromSweep :type Boolean) (SweepResult :type Hit%20Result%20Structure%20%28by%20ref%29))
  (Input|EnableInput (Game|GetPlayerController 0))
  (bind _output_get (Variables|Default|SetWithinReach true))
  (if _output_get
    (if (<= (- 1.0 (Math|Vector|DotProduct (Transformation|GetActorForwardVector OtherActor) (Math|Vector|Normalize (- (Transformation|GetActorLocation) (Transformation|GetActorLocation OtherActor))))) (Variables|Default|GetOffset))
      (Variables|Default|SetFacingResource true)
      ;[1 1 1] Remove later
      (Development|PrintString "Facing the tree" true true "(R=0.000000,G=0.000000,B=1.000000,A=1.000000)")
      (else
        (Variables|Default|SetFacingResource false)
        (Development|PrintString "Not facing the tree" true true "(R=1.000000,G=0.000000,B=0.000000,A=1.000000)")))))

(event OnComponentEndOverlap(TreeMainCollider)
  (params (OverlappedComponent :type Primitive%20Component%20Object%20Reference) (OtherActor :type Actor%20Object%20Reference) (OtherComp :type Primitive%20Component%20Object%20Reference) (OtherBodyIndex :type Integer))
  (Variables|Default|SetWithinReach false)
  (Input|DisableInput (Game|GetPlayerController 0))
  (bind _asbuilder (Utilities|Casting|CastToBuilder (stale OnComponentBeginOverlap(TreeMainCollider) OtherActor)))
  (Variables|/Game/Blueprints/Builder.Builder_C|SetisChoppingTree _asbuilder false))

(event OnClicked(ClickSurface)
  (params (TouchedComponent :type Primitive%20Component%20Object%20Reference) (ButtonPressed :type Key%20Structure))
  ;[1 1 1] Change this later? See feedback #2 by Prof. Radicke
  (bind _asbuilder (Utilities|Casting|CastToBuilder (Variables|Reference|GetBuilderRef)))
  (Default|TreeChoppingAction _asbuilder))

(event EventBeginPlay
  (Input|EnableInput (Game|GetPlayerController 0))
  (bind _outactors (Actor|GetAllActorsOfClass "/Script/Engine.Character"))
  (Variables|Reference|SetBuilderRef (Utilities|Array|Get(acopy) _outactors)))

(event Input|MouseEvents|RightMouseButton
  (params (Key :type Key%20Structure))
  (:Pressed
    (if (and (Variables|Default|GetWithinReach) (Variables|Default|GetFacingResource))
      (bind _asbuilder (Utilities|Casting|CastToBuilder (stale OnComponentBeginOverlap(TreeMainCollider) OtherActor)))
      (Variables|/Game/Blueprints/Builder.Builder_C|SetisChoppingTree _asbuilder true)
      (Variables|/Game/Blueprints/Builder.Builder_C|SetisMining _asbuilder false)
      (else
        (bind _asbuilder_2 (Utilities|Casting|CastToBuilder (stale OnComponentBeginOverlap(TreeMainCollider) OtherActor)))
        (Variables|/Game/Blueprints/Builder.Builder_C|SetisChoppingTree _asbuilder_2 false)))))

(fn ConstructionScript)