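; TreeOfLife is a damageable actor with hit points and a health bar component.
; It starts at maximum hit points, and GetDamaged subtracts from the current value without clamping or death handling.
; GetCurrentHealthPercentage returns current over maximum health as a normalized ratio.
; Each tick it rotates the health bar to face the first child component of the CameraPawn's Camera, using the pawn cached at BeginPlay.
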(event EventBeginPlay
  (bind _outactors (Actor|GetAllActorsOfClass "/Game/Blueprints/CameraPawn.CameraPawn_C"))
  (Variables|Default|SetCameraPawn (Utilities|Array|Get(acopy) _outactors))
  (Variables|Default|SetCurrentHitPoints (Variables|Default|GetMaxHitPoints)))

(event Collision|EventActorBeginOverlap
  (params (OtherActor :type Actor%20Object%20Reference)))

(event EventTick
  (params (DeltaSeconds :type Float%20%28single-precision%29))
  (bind _healthbar (Variables|Default|GetHealthBar))
  (bind _ascamera_pawn (Utilities|Casting|CastToCameraPawn (Variables|Default|GetCameraPawn)))
  (Transformation|SetWorldRotation _healthbar (Math|Rotator|FindLookatRotation (Transformation|GetWorldLocation _healthbar) (Transformation|GetWorldLocation (Components|GetChildComponent (Variables|/Game/Blueprints/CameraPawn.CameraPawn_C|GetCamera _ascamera_pawn) 0))) false false))

(fn ConstructionScript)

(fn GetDamaged
  (params (Damage :type Float%20%28single-precision%29))
  (Variables|Default|SetCurrentHitPoints (- (Variables|Default|GetCurrentHitPoints) Damage))
  (return))

(fn GetCurrentHealthPercentage
  (return (Math|Float|NormalizetoRange (/ (Variables|Default|GetCurrentHitPoints) (Variables|Default|GetMaxHitPoints)) 0.0 1.0)))