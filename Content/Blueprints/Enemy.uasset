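; Zombie enemy character Blueprint meant to run toward the TreeOfLife actor and attack it within range, though its event logic is currently disconnected.
; BeginPlay, Tick and GetHitByBullet are empty; orphaned nodes hold the target lookup, hit message and distance-based move, stop or attack decision.
; MoveZombie uses SimpleMoveToLocation, StopZombie halts movement, and Attack only prints.
; All three functions set state flags on ZombieAnimBP.
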(event Custom|GetHitByBullet)

(event EventBeginPlay)

(event EventTick
  (params (DeltaSeconds :type Float%20%28single-precision%29)))

(fn ConstructionScript)

(fn Attack
  (Development|PrintString "Attack")
  (bind _aszombie_anim_bp (Utilities|Casting|CastToZombieAnimBP (Components|SkeletalMesh|GetAnimInstance (Variables|Character|GetMesh))))
  (Variables|/Game/Zombie/ZombieAnimBP.ZombieAnimBP_C|SetisIdle _aszombie_anim_bp false)
  (Variables|/Game/Zombie/ZombieAnimBP.ZombieAnimBP_C|SetisRunning _aszombie_anim_bp false)
  (Variables|/Game/Zombie/ZombieAnimBP.ZombieAnimBP_C|SetisAttacking _aszombie_anim_bp true)
  (return))

(fn MoveZombie
  (bind _aszombie_anim_bp (Utilities|Casting|CastToZombieAnimBP (Components|SkeletalMesh|GetAnimInstance (Variables|Character|GetMesh))))
  (bind _output_get (Variables|/Game/Zombie/ZombieAnimBP.ZombieAnimBP_C|SetisIdle _aszombie_anim_bp false))
  (Variables|/Game/Zombie/ZombieAnimBP.ZombieAnimBP_C|SetisRunning _aszombie_anim_bp (not _output_get))
  (Variables|/Game/Zombie/ZombieAnimBP.ZombieAnimBP_C|SetisAttacking _aszombie_anim_bp false)
  (AI|Navigation|SimpleMovetoLocation (AI|GetAIController self) (Variables|Default|GetGoalLocation))
  (return))

(fn StopZombie
  (Components|Movement|StopMovementImmediately (Variables|Character|GetCharacterMovement))
  (bind _aszombie_anim_bp (Utilities|Casting|CastToZombieAnimBP (Components|SkeletalMesh|GetAnimInstance (Variables|Character|GetMesh))))
  (Variables|/Game/Zombie/ZombieAnimBP.ZombieAnimBP_C|SetisIdle _aszombie_anim_bp true)
  (Variables|/Game/Zombie/ZombieAnimBP.ZombieAnimBP_C|SetisRunning _aszombie_anim_bp false)
  (return))