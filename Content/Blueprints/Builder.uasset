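; Builder character that gathers rock and logs and places towers for the player.
; Tick sets BuilderAnimBP walking from goal distance and, outside build mode, runs a delayed collection macro that plays the collect animation and adds resources.
; Building uses preview actors: OnBuildTowerMesh checks the GameInstance log cost, then swaps the preview for a tower at the cursor hit.
; Only Log Tower spawns; Rock Tower and TreeChoppingAction are stubs.
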(event Custom|OnBuildTowerMesh
  ;[1 1 1] Building & Build Preview
  (if (Variables|Flags|GetcanBuild)
    (bind _asmy_game_instance (Utilities|Casting|CastToMyGameInstance (Game|GetGameInstance)))
    (if (>= (Variables|Inventory|GetLogAmount) (Variables|/Game/Blueprints/MyGameInstance.MyGameInstance_C|GetLogTowerCost _asmy_game_instance))
      (Development|PrintString (Variables|Types|GetBuildingType))
      (bind _aslog_tower_preview (Utilities|Casting|CastToLogTower_Preview (Variables|References|GetBuildingPreview)))
      (Default|DestroyPreview _aslog_tower_preview)
      (CallFunction|SpawnActualBuilding (Math|Transform|MakeTransform (.Location (Collision|BreakHitResult (.HitResult (Game|Player|GetHitResultUnderCursorbyChannel (Game|GetPlayerController 0) "TraceTypeQuery1" true)))) "0, 0, 0" "1,1,1"))
      (CallFunction|ResetBuildingPreview)
      (bind _asmy_game_instance_2 (Utilities|Casting|CastToMyGameInstance (Game|GetGameInstance)))
      (Variables|Inventory|SetLogAmount (- (Variables|Inventory|GetLogAmount) (Variables|/Game/Blueprints/MyGameInstance.MyGameInstance_C|GetLogTowerCost _asmy_game_instance_2)))
      (else
        (Development|PrintString "Not Enough Resources" true true "(R=1.000000,G=0.000000,B=0.008376,A=1.000000)")
        (CallFunction|ResetPreview)))))

(event Custom|TreeChoppingAction
  ;[1 1 1] Change this later? See feedback #2 by Prof. Radicke
  (Development|PrintString "Let the tree choppin' begin, boiz!!!")
  (if (>= (Math|Vector|VectorLength (- (Transformation|GetActorLocation) (.Location (Collision|BreakHitResult (.HitResult (Game|Player|GetHitResultUnderCursorbyChannel (Variables|References|GetCameraControllerRef) "TraceTypeQuery1" true)))))) 1.5e+02)
    _))

(event EventTick
  (params (DeltaSeconds :type Float%20%28single-precision%29))
  ;[1 1 1] Resource Collection
  (if (Variables|Flags|GetisBuildMode)
    (Variables|Flags|SetisMining false)
    (Variables|Flags|SetisChoppingTree false))
  (bind _goalreached (CallFunction|HasReachedGoal (Variables|Default|GetGoalLocation)))
  (bind _asbuilder_anim_bp (Utilities|Casting|CastToBuilderAnimBP (Components|SkeletalMesh|GetAnimInstance (Variables|Character|GetMesh))))
  (Variables|/Game/Character/BuilderAnimBP/BuilderAnimBP.BuilderAnimBP_C|SetisWalking _asbuilder_anim_bp (not _goalreached))
  (if (Variables|Flags|GetisMining)
    (Variables|Types|SetResourceType (Utilities|Array|Get(acopy) (Variables|Types|GetResourceTypes)))
    (Utilities|ResourceCollection)
    (elif (Variables|Flags|GetisChoppingTree)
      (Variables|Types|SetResourceType (Utilities|Array|Get(acopy) (Variables|Types|GetResourceTypes) 1))
      (Utilities|ResourceCollection)
      (else
        (Variables|Types|SetResourceType "")))))

(event EventBeginPlay
  (bind _returnvalue (Game|GetPlayerController 0))
  ;[1 1 1] Setup the starting location
  (Utilities|FlowControl|Sequence
    (:then_0
      (Variables|Default|SetGoalLocation (Transformation|GetActorLocation))
      (bind _ascamera_controller (Utilities|Casting|CastToCameraController _returnvalue))
      (Variables|References|SetCameraControllerRef _ascamera_controller)
      (bind _ascamera_pawn (Utilities|Casting|CastToCameraPawn (Game|Player|GetPlayerPawn 0)))
      (Variables|References|SetCameraPawnRef _ascamera_pawn)
      (Input|EnableInput _returnvalue))))

(fn ConstructionScript)

(fn SetWalkingAnim
  (params (isWalking :type Boolean))
  (bind _asbuilder_anim_bp (Utilities|Casting|CastToBuilderAnimBP (Components|SkeletalMesh|GetAnimInstance (Variables|Character|GetMesh))))
  (Variables|/Game/Character/BuilderAnimBP/BuilderAnimBP.BuilderAnimBP_C|SetisWalking _asbuilder_anim_bp isWalking))

(fn HasReachedGoal
  (params (GoalPosition :type Vector))
  (return (<= (Math|Vector|VectorLength (- GoalPosition (Transformation|GetActorLocation))) 125.0)))

(fn CollectResource
  (params (Type :type String))
  (switch string Type
    (:Rock
      (Development|PrintString Type))
    (:Tree
      (Development|PrintString Type)))
  (bind _asbuilder_anim_bp (Utilities|Casting|CastToBuilderAnimBP (Components|SkeletalMesh|GetAnimInstance (Variables|Character|GetMesh))))
  (Variables|/Game/Character/BuilderAnimBP/BuilderAnimBP.BuilderAnimBP_C|SetisCollecting _asbuilder_anim_bp true)
  (return))

(fn ResetAnimations
  (params (AnimObject :type Object%20Object%20Reference))
  (bind _asbuilder_anim_bp (Utilities|Casting|CastToBuilderAnimBP AnimObject))
  (switch string (Variables|Types|GetResourceType)
    (:Default
      (Development|PrintString "No resource"))
    (:Rock
      (bind _output_get (Variables|/Game/Character/BuilderAnimBP/BuilderAnimBP.BuilderAnimBP_C|SetisCollecting _asbuilder_anim_bp false))
      (Variables|Flags|SetisMining _output_get))
    (:Tree
      (bind _output_get_2 (Variables|/Game/Character/BuilderAnimBP/BuilderAnimBP.BuilderAnimBP_C|SetisCollecting _asbuilder_anim_bp false))
      (Variables|Flags|SetisChoppingTree _output_get_2)))
  (return))

(fn SetSightDistance
  (return (+ (Variables|Default|GetSightDistance) (Variables|/Script/Engine.SpringArmComponent|GetTargetArmLength (Variables|/Game/Blueprints/CameraPawn.CameraPawn_C|GetSpringArm (Variables|References|GetCameraPawnRef))))))

(fn SpawnPreviewBuilding
  (params (SpawnTransform :type Transform) (BuildingType :type String))
  (switch string BuildingType
    (:LogTower
      (Development|PrintString "Spawning LogTower")
      (bind _returnvalue (Game|SpawnActorfromClass "/Game/Blueprints/Buildings/Defense/LogTower_Preview.LogTower_Preview_C" SpawnTransform "Undefined" 0 0))
      (Variables|Types|SetBuildingType (Utilities|Array|Get(acopy) (Variables|Types|GetBuildingTypes)))
      (Variables|References|SetBuildingPreview _returnvalue)
      (return))
    (:RockTower
      (Development|PrintString "Spawning RockTower"))))

(fn ResetBuildingPreview
  (Variables|References|SetBuildingPreview 0)
  (Variables|Flags|SetisBuildMode false)
  (Variables|Types|SetBuildingType "")
  (Variables|Flags|SetcanBuild false))

(fn SpawnActualBuilding
  (params (SpawnTransform :type Transform))
  (switch string (Variables|Types|GetBuildingType)
    (:Default
      (Development|PrintString "ERROR" true true "(R=0.218750,G=0.002110,B=0.000000,A=1.000000)"))
    (:LogTower
      (Development|PrintString "Spawning Log Tower")
      (Game|SpawnActorfromClass "/Game/Blueprints/Buildings/Defense/LogTower.LogTower_C" SpawnTransform "Undefined" 0 0)
      (return))))

(fn ResetPreview
  (bind _aslog_tower_preview (Utilities|Casting|CastToLogTower_Preview (Variables|References|GetBuildingPreview)))
  (Default|DestroyPreview _aslog_tower_preview)
  (CallFunction|ResetBuildingPreview))

(fn ResourceCollect
  (params (Hit :type Hit%20Result%20Structure) (ResourceLocation :type Vector))
  (while (>= (Math|Vector|VectorLength (- (Transformation|GetActorLocation) ResourceLocation)) 1e+02)
    (Default|MoveBuilder (Variables|References|GetCameraControllerRef) Hit))
  (Components|Movement|StopMovementImmediately (Variables|Character|GetCharacterMovement))
  (CallFunction|CollectResource (Variables|Types|GetResourceType))
  (return))