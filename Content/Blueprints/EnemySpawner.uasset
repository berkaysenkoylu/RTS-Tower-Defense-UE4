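; Enemy spawner Blueprint that creates Zombie AI pawns at randomly chosen SpawnPoint actors.
; BeginPlay caches every SpawnPoint in the level into SpawnLocations.
; The CanSpawnEnemy event waits a short delay, then calls SpawnEnemy, which spawns one Zombie using the location and rotation from GetRandomSpawnTransform.
; Nothing in this Blueprint triggers CanSpawnEnemy or loops it, so each spawn depends on an outside call.
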(event Custom|CanSpawnEnemy
  (Utilities|FlowControl|Delay 1.5)
  (CallFunction|SpawnEnemy))

(event EventBeginPlay
  (bind _outactors (Actor|GetAllActorsOfClass "/Game/Blueprints/SpawnPoint.SpawnPoint_C"))
  (Variables|Default|SetSpawnLocations _outactors))

(fn ConstructionScript)

(fn SpawnEnemy
  (bind _spawntransform (CallFunction|GetRandomSpawnTransform))
  (AI|SpawnAIFromClass "/Game/Blueprints/Zombie.Zombie_C" 0 (.location _spawntransform) (.rotation _spawntransform) false)
  (return))

(fn GetRandomSpawnTransform
  (return (Transformation|GetActorTransform (Utilities|Array|Get(acopy) (Variables|Default|GetSpawnLocations) (Math|Random|RandomInteger (Utilities|Array|Length (Variables|Default|GetSpawnLocations)))))))