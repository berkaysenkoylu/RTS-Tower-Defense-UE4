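; DayNightCycle Blueprint that animates a day-night cycle and triggers enemy spawning at night.
; On BeginPlay it caches the first DirectionalLight and the first EnemySpawner found in the level.
; Each Tick it rotates the light's pitch by Speed scaled with delta time.
; While the pitch is above zero up to 90 degrees (light pointing upward), it calls CanSpawnEnemy on the spawner every frame.
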(event EventTick
  (params (DeltaSeconds :type Float%20%28single-precision%29))
  (Transformation|AddActorLocalRotation (Variables|Default|GetLightSource) (Math|Rotator|MakeRotator 0.0 (* DeltaSeconds (Variables|Default|GetSpeed)) 0.0) false false)
  (bind _output_get (Variables|Default|SetPitchAngle (.pitch (Transformation|GetActorRotation (Variables|Default|GetLightSource)))))
  (if (and (> _output_get 0.0) (<= _output_get 9e+01))
    (bind _asenemy_spawner (Utilities|Casting|CastToEnemySpawner (Variables|Default|GetEnemySpawner)))
    (Default|CanSpawnEnemy _asenemy_spawner)))

(event EventBeginPlay
  (bind _outactors (Actor|GetAllActorsOfClass "/Script/Engine.DirectionalLight"))
  (Variables|Default|SetLightSource (Utilities|Array|Get(acopy) _outactors))
  (bind _outactors_2 (Actor|GetAllActorsOfClass "/Game/Blueprints/EnemySpawner.EnemySpawner_C"))
  (Variables|Default|SetEnemySpawner (Utilities|Array|Get(acopy) _outactors_2)))

(fn ConstructionScript)